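; BP_Tunnel is a segment of an endless tunnel with a rotating holed wall the player must pass through.
; Entering the trigger asks TunnelSpawner for another tunnel and adds score, while hitting the wall deducts score and notifies the player.
; Exiting updates score display and player velocity, then destroys the segment, its life pack and its enemies.
; RandomizeWall varies hole mesh, starting roll and spin speed, but is not called within this Blueprint.
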(event OnComponentBeginOverlap(TriggerZone)
  (params (OverlappedComponent :type Primitive%20Component%20Object%20Reference) (OtherActor :type Actor%20Object%20Reference) (OtherComp :type Primitive%20Component%20Object%20Reference) (OtherBodyIndex :type Integer) (bFromSweep :type Boolean) (SweepResult :type Hit%20Result%20Structure%20%28by%20ref%29))
  ;[1 1 1] spawn tunnel
  (bind _asbp_player (Utilities|Casting|CastToBP_Player OtherActor))
  (Default|SpawnTunnelatSpawnPoint (Variables|Default|GetTunnelSpawner))
  (Variables|/Game/InfiniteMatrix/Blueprints/BP_Player.BP_Player_C|SetScore _asbp_player (+ 1 (Variables|/Game/InfiniteMatrix/Blueprints/BP_Player.BP_Player_C|GetScore _asbp_player))))

(event OnComponentBeginOverlap(WallMesh)
  (params (OverlappedComponent :type Primitive%20Component%20Object%20Reference) (OtherActor :type Actor%20Object%20Reference) (OtherComp :type Primitive%20Component%20Object%20Reference) (OtherBodyIndex :type Integer) (bFromSweep :type Boolean) (SweepResult :type Hit%20Result%20Structure%20%28by%20ref%29))
  ;[1 1 1] Player hit mesh
  (if (Class|GameplayStatics|ObjectIsA OtherActor "/Game/InfiniteMatrix/Blueprints/BP_Player.BP_Player_C")
    (bind _asbp_player (Utilities|Casting|CastToBP_Player OtherActor))
    (Default|WhenHitWall _asbp_player)
    (Variables|/Game/InfiniteMatrix/Blueprints/BP_Player.BP_Player_C|SetScore _asbp_player (+ -1 (Variables|/Game/InfiniteMatrix/Blueprints/BP_Player.BP_Player_C|GetScore _asbp_player)))))

(event OnComponentEndOverlap(TriggerZone)
  (params (OverlappedComponent :type Primitive%20Component%20Object%20Reference) (OtherActor :type Actor%20Object%20Reference) (OtherComp :type Primitive%20Component%20Object%20Reference) (OtherBodyIndex :type Integer))
  (bind _lifepack (Variables|Default|GetLifePack))
  ;[1 1 1] Update score and velocity after leaving mesh
  (if (Class|GameplayStatics|ObjectIsA OtherActor "/Game/InfiniteMatrix/Blueprints/BP_Player.BP_Player_C")
    (Utilities|FlowControl|Sequence
      (:then_0
        (bind _asbp_player (Utilities|Casting|CastToBP_Player OtherActor))
        (Default|UpdateScore (Variables|/Game/InfiniteMatrix/Blueprints/BP_Player.BP_Player_C|GetScoreWidget _asbp_player) (Variables|/Game/InfiniteMatrix/Blueprints/BP_Player.BP_Player_C|GetScore _asbp_player))
        (Default|UpdateVelocity _asbp_player)
        (Actor|DestroyActor))
      (:then_1
        ;[1 1 1] breaking life pack
        (Utilities|IsValid _lifepack
          (:Is%20Valid
            (Actor|DestroyActor _lifepack))))
      (:then_2
        ;[1 1 1] breaking enermy
        (bind _outactors (Actor|GetAllActorsOfClass "/Game/InfiniteMatrix/Blueprints/BP_Enermy.BP_Enermy_C"))
        (for _array_element _outactors
          (if (== self (Variables|/Game/InfiniteMatrix/Blueprints/BP_Enermy.BP_Enermy_C|GetmyTunnel _array_element))
            (Actor|DestroyActor _array_element)))))))

(event EventBeginPlay)

(event EventTick
  (params (DeltaSeconds :type Float%20%28single-precision%29))
  ;[1 1 1] mesh rotation
  (Transformation|AddLocalRotation (Variables|Default|GetWallMesh) (Math|Rotator|MakeRotator (* DeltaSeconds (Variables|Default|GetRotateSpeed)) 0.0 0.0) false false))

(fn ConstructionScript)

(fn RandomizeWall
  (Components|StaticMesh|SetStaticMesh (Variables|Default|GetWallMesh) (Utilities|Select :Index (Math|Random|RandomIntegerinRange 0 3) :Option%200 "/Game/InfiniteMatrix/Meshes/SM_Hole_01.SM_Hole_01" :Option%201 "/Game/InfiniteMatrix/Meshes/SM_Hole_02.SM_Hole_02" :Option%202 "/Game/InfiniteMatrix/Meshes/SM_Hole_03.SM_Hole_03" :Option%203 "/Game/InfiniteMatrix/Meshes/SM_Hole_04.SM_Hole_04"))
  (Transformation|AddLocalRotation (Variables|Default|GetWallMesh) (Math|Rotator|MakeRotator (Math|Random|RandomFloatinRange 0.0 3.6e+02) 0.0 0.0) false false)
  ;[1 1 1] Randomize rotation speed
  (Variables|Default|SetRotateSpeed (* (Variables|Default|GetRotateSpeed) (Math|Random|RandomFloatinRange 0.1 1.5))))