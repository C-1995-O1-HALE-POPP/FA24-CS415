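; BP_TunnelSpawner builds the chain of BP_Tunnel segments the player travels through and populates each one.
; On BeginPlay it destroys existing tunnels, then spawns up to MaxTunnelAlive segments, starting at the player pawn and chaining at the newest segment's SpawnPoint.
; Each segment gets a spawner back-reference, randomized walls, and weighted-random rolls for a life pack and several enemies, which position themselves through SpawnMe.
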(event EventBeginPlay
  (CallFunction|SpawnInitialTunnels))

(event Collision|EventActorBeginOverlap
  (params (OtherActor :type Actor%20Object%20Reference)))

(event EventTick
  (params (DeltaSeconds :type Float%20%28single-precision%29)))

(fn ConstructionScript)

(fn SpawnTunnel
  (params (SpawnLocation :type Vector))
  (bind _returnvalue (Game|SpawnActorfromClass "/Game/InfiniteMatrix/Blueprints/BP_Tunnel.BP_Tunnel_C" (Math|Transform|MakeTransform SpawnLocation "0, 0, 0" "1.000000,1.000000,1.000000") "Undefined" "MultiplyWithRoot" 0 0))
  (bind _output_get (Variables|Default|SetNewestTunnel _returnvalue))
  (Variables|/Game/InfiniteMatrix/Blueprints/BP_Tunnel.BP_Tunnel_C|SetTunnelSpawner _output_get self)
  (Default|RandomizeWall _output_get)
  (CallFunction|SpawnLifePack)
  (CallFunction|SpawnEnermy))

(fn SpawnTunnelatSpawnPoint
  (CallFunction|SpawnTunnel (Transformation|GetWorldLocation (Variables|/Game/InfiniteMatrix/Blueprints/BP_Tunnel.BP_Tunnel_C|GetSpawnPoint (Variables|Default|GetNewestTunnel)))))

(fn SpawnInitialTunnels
  (Utilities|FlowControl|Sequence
    (:then_0
      (bind _outactors (Actor|GetAllActorsOfClass "/Game/InfiniteMatrix/Blueprints/BP_Tunnel.BP_Tunnel_C"))
      (for _array_element _outactors
        (Actor|DestroyActor _array_element)))
    (:then_1
      (for _index (range 0 (- (Variables|Default|GetMaxTunnelAlive) 1))
        (Utilities|IsValid (Variables|Default|GetNewestTunnel)
          (:Is%20Valid
            (CallFunction|SpawnTunnelatSpawnPoint))
          (:Is%20Not%20Valid
            (CallFunction|SpawnTunnel (Transformation|GetActorLocation (Game|Player|GetPlayerPawn 0)))))))))

(fn SpawnLifePack
  (bind _newesttunnel (Variables|Default|GetNewestTunnel))
  (if (Math|Random|RandomBoolwithWeight 0.9)
    (bind _returnvalue (Game|SpawnActorfromClass "/Game/InfiniteMatrix/Blueprints/BP_LifePack.BP_LifePack_C" (Math|Transform|MakeTransform "0, 0, 0" "0, 0, 0" "1.000000,1.000000,1.000000") "Undefined" "MultiplyWithRoot" 0 0))
    (bind _output_get (Variables|/Game/InfiniteMatrix/Blueprints/BP_Tunnel.BP_Tunnel_C|SetLifePack _newesttunnel _returnvalue))
    (Variables|/Game/InfiniteMatrix/Blueprints/BP_LifePack.BP_LifePack_C|SetmyTunnel _output_get _newesttunnel)
    (Default|SpawnMe _output_get)))

(fn GetRandomVector
  (return "0, 0, 0"))

(fn SpawnEnermy
  (for _index (range 0 (+ (Variables|/Game/InfiniteMatrix/Blueprints/BP_Tunnel.BP_Tunnel_C|GetMaxEnermyPerTunnel (Variables|Default|GetNewestTunnel)) -1))
    (if (Math|Random|RandomBoolwithWeight 0.9)
      (bind _returnvalue (Game|SpawnActorfromClass "/Game/InfiniteMatrix/Blueprints/BP_Enermy.BP_Enermy_C" (Math|Transform|MakeTransform "0, 0, 0" "0, 0, 0" "1.000000,1.000000,1.000000") "Undefined" "MultiplyWithRoot" 0 0))
      (Variables|/Game/InfiniteMatrix/Blueprints/BP_Enermy.BP_Enermy_C|SetmyTunnel _returnvalue (Variables|Default|GetNewestTunnel))
      (Default|SpawnMe _returnvalue))))