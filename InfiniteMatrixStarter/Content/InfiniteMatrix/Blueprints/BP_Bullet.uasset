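; BP_Bullet is a projectile that travels along world X and destroys life packs and enemies to score points for its shooter.
; Tick moves it by Speed scaled by delta time, with sweep enabled.
; On overlap, a tunnel destroys only the bullet.
; A life pack or enemy is destroyed with it, raising FromWho's Score, decrementing its Bullet count and refreshing both widgets.
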(event OnComponentBeginOverlap(SM_Bullet)
  (params (OverlappedComponent :type Primitive%20Component%20Object%20Reference) (OtherActor :type Actor%20Object%20Reference) (OtherComp :type Primitive%20Component%20Object%20Reference) (OtherBodyIndex :type Integer) (bFromSweep :type Boolean) (SweepResult :type Hit%20Result%20Structure%20%28by%20ref%29))
  (bind _fromwho (Variables|Default|GetFromWho))
  (if (Class|GameplayStatics|ObjectIsA OtherActor "/Game/InfiniteMatrix/Blueprints/BP_Tunnel.BP_Tunnel_C")
    (Actor|DestroyActor)
    (elif (Class|GameplayStatics|ObjectIsA OtherActor "/Game/InfiniteMatrix/Blueprints/BP_LifePack.BP_LifePack_C")
      (Actor|DestroyActor OtherActor :!label _label)
      (bind _result (Math|Integer|IncrementInt (Variables|/Game/InfiniteMatrix/Blueprints/BP_Player.BP_Player_C|GetScore _fromwho))
        (:%20%20
          (bind _output_get (Variables|/Game/InfiniteMatrix/Blueprints/BP_Player.BP_Player_C|SetScore _fromwho _result))
          (Default|UpdateScore (Variables|/Game/InfiniteMatrix/Blueprints/BP_Player.BP_Player_C|GetScoreWidget _fromwho) _output_get)
          (bind _result_2 (Math|Integer|DecrementInt (Variables|/Game/InfiniteMatrix/Blueprints/BP_Player.BP_Player_C|GetBullet _fromwho))
            (:%20%20
              (bind _output_get_2 (Variables|/Game/InfiniteMatrix/Blueprints/BP_Player.BP_Player_C|SetBullet _fromwho _result_2))
              (Default|UpdateBullet (Variables|/Game/InfiniteMatrix/Blueprints/BP_Player.BP_Player_C|GetBulletWidget _fromwho) _output_get_2 (Variables|/Game/InfiniteMatrix/Blueprints/BP_Player.BP_Player_C|GetMaxBullet _fromwho))
              (Actor|DestroyActor)))))
      (elif (Class|GameplayStatics|ObjectIsA OtherActor "/Game/InfiniteMatrix/Blueprints/BP_Enermy.BP_Enermy_C")
        (goto _label)))))

(event EventTick
  (params (DeltaSeconds :type Float%20%28single-precision%29))
  (Transformation|AddActorWorldOffset (Math|Vector|MakeVector (* DeltaSeconds (Variables|Default|Getspeed)) 0.0 0.0) true))

(fn ConstructionScript)