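; BP_LifePack is a drifting, spinning pickup that gives the player health and score.
; A hit by the player pawn adds one Health and one Score, updates both widgets and destroys the pack.
; Overlapping a BP_Tunnel calls SpawnMe, which moves the pack to a random offset from MyTunnel's SpawnPoint.
; SetPhysics then randomizes the MoveIndex transform, which Tick applies as linear and angular velocity without physics simulation.
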(event OnComponentHit(SM_LifePack)
  (params (HitComponent :type Primitive%20Component%20Object%20Reference) (OtherActor :type Actor%20Object%20Reference) (OtherComp :type Primitive%20Component%20Object%20Reference) (NormalImpulse :type Vector :default "0, 0, 0") (Hit :type Hit%20Result%20Structure%20%28by%20ref%29))
  (bind _returnvalue (Game|Player|GetPlayerPawn 0))
  (if (== OtherActor _returnvalue)
    (bind _asbp_player (Utilities|Casting|CastToBP_Player _returnvalue))
    (Utilities|FlowControl|Sequence
      (:then_0
        ;[1 1 1] Life
        (bind _output_get (Variables|/Game/InfiniteMatrix/Blueprints/BP_Player.BP_Player_C|SetHealth _asbp_player (+ (Variables|/Game/InfiniteMatrix/Blueprints/BP_Player.BP_Player_C|GetHealth _asbp_player) 1)))
        (Default|UpdateLife (Variables|/Game/InfiniteMatrix/Blueprints/BP_Player.BP_Player_C|GetHealthWidget _asbp_player) _output_get (Variables|/Game/InfiniteMatrix/Blueprints/BP_Player.BP_Player_C|GetMaxHealth _asbp_player) true))
      (:then_1
        (bind _result (Math|Integer|IncrementInt (Variables|/Game/InfiniteMatrix/Blueprints/BP_Player.BP_Player_C|GetScore _asbp_player))
          (:%20%20
            (bind _output_get_2 (Variables|/Game/InfiniteMatrix/Blueprints/BP_Player.BP_Player_C|SetScore _asbp_player _result))
            (Default|UpdateScore (Variables|/Game/InfiniteMatrix/Blueprints/BP_Player.BP_Player_C|GetScoreWidget _asbp_player) _output_get_2))))
      (:then_2
        (Actor|DestroyActor)))))

(event OnComponentBeginOverlap(SM_LifePack)
  (params (OverlappedComponent :type Primitive%20Component%20Object%20Reference) (OtherActor :type Actor%20Object%20Reference) (OtherComp :type Primitive%20Component%20Object%20Reference) (OtherBodyIndex :type Integer) (bFromSweep :type Boolean) (SweepResult :type Hit%20Result%20Structure%20%28by%20ref%29))
  (if (Class|GameplayStatics|ObjectIsA OtherActor "/Game/InfiniteMatrix/Blueprints/BP_Tunnel.BP_Tunnel_C")
    (CallFunction|SpawnMe)))

(event EventBeginPlay)

(event Collision|EventActorBeginOverlap
  (params (OtherActor :type Actor%20Object%20Reference)))

(event EventTick
  (params (DeltaSeconds :type Float%20%28single-precision%29))
  (bind _moveindex (Variables|Default|GetmoveIndex))
  (Transformation|AddActorWorldOffset (Math|Vector|MakeVector (* (.x (.location _moveindex)) DeltaSeconds) (* (.y (.location _moveindex)) DeltaSeconds) (* (.z (.location _moveindex)) DeltaSeconds)))
  (Class|Actor|AddActorWorldRotation (Math|Rotator|MakeRotator (* (.roll (.rotation _moveindex)) DeltaSeconds) (* (.pitch (.rotation _moveindex)) DeltaSeconds) (* (.yaw (.rotation _moveindex)) DeltaSeconds))))

(fn ConstructionScript)

(fn SetPhysics
  (bind _maxrotationspeed (Variables|Default|GetMaxRotationSpeed))
  (bind _maxmovespeed (Variables|Default|GetMaxMoveSpeed))
  (bind _returnvalue (- 0.0 _maxrotationspeed))
  (bind _returnvalue_2 (- 0.0 _maxmovespeed))
  (bind _returnvalue_3 (Math|Random|RandomFloatinRange _returnvalue _maxrotationspeed))
  (bind _returnvalue_4 (Math|Random|RandomFloatinRange _returnvalue _maxrotationspeed))
  (bind _returnvalue_5 (Math|Random|RandomFloatinRange _returnvalue _maxrotationspeed))
  (Variables|Default|SetmoveIndex (Math|Transform|MakeTransform (Math|Vector|MakeVector (* (Math|Random|RandomFloatinRange _returnvalue_2 _maxmovespeed) 5.0) (Math|Random|RandomFloatinRange _returnvalue_2 _maxmovespeed) (Math|Random|RandomFloatinRange _returnvalue_2 _maxmovespeed)) (Math|Rotator|MakeRotator _returnvalue_3 _returnvalue_4 _returnvalue_5) "1.000000,1.000000,1.000000"))
  (Transformation|AddActorLocalRotation (Math|Rotator|MakeRotator _returnvalue_3 _returnvalue_4 _returnvalue_5) false false))

(fn SpawnMe
  (bind _returnvalue (Math|Random|RandomFloatinRange -2e+02 2e+02))
  (bind _returnvalue_2 (Math|Random|RandomFloatinRange -2e+02 2e+02))
  (bind _mytunnel (Variables|Default|GetmyTunnel))
  (Utilities|IsValid _mytunnel
    (:Is%20Valid
      (if (< (+ (Math|Float|Square _returnvalue) (Math|Float|Square _returnvalue_2)) 2.5e+05)
        (Transformation|SetActorLocation (+ (Transformation|GetWorldLocation (Variables|/Game/InfiniteMatrix/Blueprints/BP_Tunnel.BP_Tunnel_C|GetSpawnPoint _mytunnel)) (Math|Vector|MakeVector (Math|Random|RandomFloatinRange -2e+03 -5e+02) _returnvalue _returnvalue_2)) false false)
        (CallFunction|SetPhysics)
        (else
          (CallFunction|SpawnMe))))))